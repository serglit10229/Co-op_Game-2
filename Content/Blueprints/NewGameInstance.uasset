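; Game instance that hosts multiplayer lobbies through an Advanced Session node.
; CreateLobby stores the server name, slot count and LAN choice, then creates a session for the first player controller with those values.
; Name and LAN flag are also passed as extra session settings.
; On success it opens the "New" level as a listen server; no failure branch is shown.
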(event Custom|CreateLobby
  (params (ServerName :type String) (ServerSlots :type Integer) (ServerMethod_Lan :type Boolean))
  (Variables|Default|SetServerName ServerName)
  (Variables|Default|SetServerSlots ServerSlots)
  (Variables|Default|SetServerMethod_Lan ServerMethod_Lan)
  (|AdvancedSession (Utilities|Array|MakeArray (Class|AdvancedSessionsLibrary|MakeLiteralSessionPropertyString "NAME" (Variables|Default|GetServerName)) "" (Class|AdvancedSessionsLibrary|MakeLiteralSessionPropertyBool "LAN" (Variables|Default|GetServerMethod_Lan)) "") (Game|GetPlayerController 0) (Variables|Default|GetServerSlots) 0 (Variables|Default|GetServerMethod_Lan) true false true true false false false true
    (:OnSuccess
      (Game|OpenLevel(byName) "New" true "listen"))))